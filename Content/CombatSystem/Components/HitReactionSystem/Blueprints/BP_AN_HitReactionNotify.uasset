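; Anim notify, shown as "Hit Reaction", that loads an animation's hit parameters into the owning actor's combat hit reaction component.
; When fired, it finds the owner's HitReactionComponent and passes it the notify's air-launch flag, damage, pushback, sound, Niagara effect and camera shake settings.
; It then removes the notify's stamina cost through the same component.
; The separate HitParticleFX variable is unused.
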(fn `GetNotifyName`
  (returns (ReturnValue :type String))
  (return "Hit Reaction"))

(fn `Received_Notify`
  (params (MeshComp :type "SkeletalMeshComponent Object Reference") (Animation :type "AnimSequenceBase Object Reference") (EventReference :type "AnimNotifyEventReference Structure (by ref)"))
  (returns (ReturnValue :type Boolean))
  (bind _returnvalue (`Actor.GetComponentByClass` (`ActorComponent.GetOwner` MeshComp) "/Script/HacknSlash.HitReactionComponent"))
  (`/Engine/EditorBlueprintResources/StandardMacros.IsValid` _returnvalue
    (:`Is Valid`
      (message `HitReactionInterface.SetHitReaction` _returnvalue (`self.bIsAirLaunchAttack`) (`self.Damage`) (`self.bHitPushBack`) (`self.PushBackDistance`) (`self.HitSFX`) (`self.Hit Niagara FX`) (`self.CameraShake`) (`self.CameraShakeScale`))
      (`HitReactionComponent.RemoveStamina` _returnvalue (`self.StaminaCost`))
      (return false))))