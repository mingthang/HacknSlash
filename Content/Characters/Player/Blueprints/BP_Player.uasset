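; BP_Player is the player character Blueprint, handling the HUD and both dealing and receiving melee-style hit damage.
; It creates WBP_HUD on BeginPlay and refreshes the stamina bar every Tick.
; HitboxComponent hits apply point damage using HitReactionComponent's damage value.
; Incoming point damage drains stamina and triggers a hit reaction in the None and Attack states, resetting ComboBufferComponent first when attacking.
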(event `self.ReceiveBeginPlay`
  (bind _returnvalue (`|CreateWidget` "/Game/CombatSystem/UI/WBP_HUD.WBP_HUD_C"))
  (bind _output_get (set `self.HUDWidget` _returnvalue))
  (`UserWidget.AddToViewport` _output_get 0)
  (`/Game/CombatSystem/UI/WBP_HUD.UpdateHealthBar` _output_get)
  (`/Game/CombatSystem/UI/WBP_HUD.UpdateStaminaBar` _output_get))

(event `self.ReceiveTick`
  (params (DeltaSeconds :type "Float (single-precision)"))
  (`/Game/CombatSystem/UI/WBP_HUD.UpdateStaminaBar` (`self.HUDWidget`)))

(event `self.HitboxComponent.OnHitResult`
  (params (HitResult :type "HitResult Structure (by ref)"))
  (bind (_bblockinghit _binitialoverlap _time _distance _location _impactpoint _normal _impactnormal _physmat _hitactor _hitcomponent _hitbonename _bonename _hititem _elementindex _faceindex _tracestart) (`GameplayStatics.BreakHitResult` HitResult))
  ; Apply Damage On Hit
  (`GameplayStatics.ApplyPointDamage` _hitactor (`HitReactionComponent.GetDamage` (`self.HitReactionComponent`)) _tracestart HitResult (`self.GetController` self) self))

(event `self.ReceivePointDamage`
  (params (Damage :type "Float (single-precision)") (DamageType :type "DamageType Object Reference") (HitLocation :type "Vector Structure") (HitNormal :type "Vector Structure") (HitComponent :type "PrimitiveComponent Object Reference") (BoneName :type Name) (ShotFromDirection :type "Vector Structure") (InstigatedBy :type "Controller Object Reference") (DamageCauser :type "Actor Object Reference") (HitInfo :type "HitResult Structure (by ref)"))
  ; Event Taking Damage
  (`HitReactionComponent.RemoveStamina` (`self.HitReactionComponent`) 20.0)
  (switch `EPlayerState` (`self.GetCurrentState` self)
    (:`None`
      _)
    (:`Attack`
      (`ComboBufferComponent.OnResetCombo` (`self.ComboBufferComponent`))))
  (`HitReactionComponent.OnHitReaction` (`self.HitReactionComponent`) Damage DamageCauser HitInfo "Player"))

(fn `UserConstructionScript`)