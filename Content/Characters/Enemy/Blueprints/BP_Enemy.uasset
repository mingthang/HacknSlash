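; Enemy character Blueprint that deals and receives point damage and shows a health bar widget.
; On BeginPlay it binds the WBP_EnemyHealthBar widget to itself and caches it.
; Hitbox component hits apply point damage using the amount from HitReactionComponent.
; Incoming point damage goes to HitReactionComponent with an "Enemy" tag, then refreshes the health bar.
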(event `self.ReceiveBeginPlay`
  ; Begin Play
  (bind _aswbp_health_bar (cast `/Game/CombatSystem/UI/WBP_EnemyHealthBar` (`WidgetComponent.GetWidget` (`self.WidgetHealthBar`))))
  (set `/Game/CombatSystem/UI/WBP_EnemyHealthBar.EnemyOwner` self _aswbp_health_bar)
  (`/Game/CombatSystem/UI/WBP_EnemyHealthBar.UpdateHealth` _aswbp_health_bar)
  (set `self.HealthBar` _aswbp_health_bar))

(event `self.HitboxComponent.OnHitResult`
  (params (HitResult :type "HitResult Structure (by ref)"))
  (bind (_bblockinghit _binitialoverlap _time _distance _location _impactpoint _normal _impactnormal _physmat _hitactor _hitcomponent _hitbonename _bonename _hititem _elementindex _faceindex _tracestart) (`GameplayStatics.BreakHitResult` HitResult))
  ; Apply Damage On Hit
  (`GameplayStatics.ApplyPointDamage` _hitactor (`HitReactionComponent.GetDamage` (`self.HitReactionComponent`)) _tracestart HitResult (`self.GetController` self) self))

(event `self.ReceivePointDamage`
  (params (Damage :type "Float (single-precision)") (DamageType :type "DamageType Object Reference") (HitLocation :type "Vector Structure") (HitNormal :type "Vector Structure") (HitComponent :type "PrimitiveComponent Object Reference") (BoneName :type Name) (ShotFromDirection :type "Vector Structure") (InstigatedBy :type "Controller Object Reference") (DamageCauser :type "Actor Object Reference") (HitInfo :type "HitResult Structure (by ref)"))
  ; Event Taking Damage
  (`HitReactionComponent.OnHitReaction` (`self.HitReactionComponent`) Damage DamageCauser HitInfo "Enemy")
  (`/Game/CombatSystem/UI/WBP_EnemyHealthBar.UpdateHealth` (`self.HealthBar`)))

(fn `UserConstructionScript`)