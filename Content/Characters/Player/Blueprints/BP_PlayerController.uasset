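; Player controller Blueprint that sets up the controlled pawn's combo system and handles pausing.
; On BeginPlay, for the local controller only, it passes the pawn's skeletal mesh to its ComboBufferComponent to initialize weapon states.
; A direct P key press toggles the game's paused state.
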(event `self.ReceiveBeginPlay`
  (bind _returnvalue (`self.K2_GetPawn`))
  (if (`self.IsLocalPlayerController`)
    (`ComboBufferComponent.InitWeaponStates` (`self.GetComponentByClass` _returnvalue "/Script/HacknSlash.ComboBufferComponent") (`self.GetComponentByClass` _returnvalue "/Script/Engine.SkeletalMeshComponent"))))

(event `Key|P` :paused true
  (params (Key :type "Key Structure"))
  (:`Pressed`
    (if (`GameplayStatics.IsGamePaused`)
      (`GameplayStatics.SetGamePaused` false)
      (else
        (`GameplayStatics.SetGamePaused` true)))))

(fn `UserConstructionScript`)